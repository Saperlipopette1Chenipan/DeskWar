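; AC_Spam is a component for a key-spam prompt that creates WBP_SPam on screen with a random press target.
; Space presses raise the clamped count and progress bar, but the completion branch is hardwired true, so the first press reports success and the target comparison is unused.
; Releasing any key restarts a short retriggerable delay that resets progress and reports failure.
; Both outcomes call CallCompleted, then remove the widget and component.
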(event `self.ReceiveBeginPlay`
  (bind _returnvalue (`|GenericCreateObject` "/Game/HUD_Game/Spam_Bar/WBP_SPam.WBP_SPam_C"))
  (set `self.WidgetReference` _returnvalue)
  (`UserWidget.AddToViewport` (`self.WidgetReference`) 0)
  (set `self.AmountNeeded` (`KismetMathLibrary.RandomFloatInRange` 10.0 15.0))
  (set `self.keyPressed` "SpaceBar")
  (`TextBlock.SetText` (`/Game/HUD_Game/Spam_Bar/WBP_SPam.SpamText` (`self.WidgetReference`)) (`|FormatText` "Spam {Key}" (`KismetInputLibrary.Key_GetDisplayName` (`self.keyPressed`))))
  (`self.UpdateProgressBar`))

(event `Press Key`
  (set `self.AmountPressed` (`KismetMathLibrary.FClamp` (+ (`self.AmountPressed`) 1.0) 0.0 (`self.AmountNeeded`)))
  (`self.UpdateProgressBar`)
  (if true
    (`self.Completed` true)
    (`self.Destroy`)))

(event `Release Key`
  (`KismetSystemLibrary.RetriggerableDelay` 0.8)
  (`self.On Failed`))

(event `On Failed`
  (set `self.AmountPressed` 0.0)
  (`self.UpdateProgressBar`)
  (`self.Completed` false)
  (`self.Destroy`))

(event `Destroy`
  (bind _widgetreference (`self.WidgetReference`)
    (:`then`
      (`Widget.RemoveFromParent` _widgetreference))
    (:`else`
      _))
  (`self.K2_DestroyComponent`))

(event `Key|AnyKey`
  (params (Key :type "Key Structure"))
  (:`Pressed`
    (if (== Key (`self.keyPressed`))
      (`self.Press Key`)))
  (:`Released`
    (`self.Release Key`)))

(fn `UpdateProgressBar`
  (`ProgressBar.SetPercent` (`/Game/HUD_Game/Spam_Bar/WBP_SPam.SpamBar` (`self.WidgetReference`)) (/ (`self.AmountPressed`) (`self.AmountNeeded`))))