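; Player 1's GrosSac character Blueprint, whose graph only handles UI widgets.
; On BeginPlay it creates and stores the PFC and PLT loading screens and the hub score widget without displaying them, then shows the main menu.
; Hard-coded keys manage the screen: I removes all widgets, and B removes all widgets and shows a newly created WBP_Sarb.
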(event `self.ReceiveBeginPlay`
  (bind _returnvalue (`|CreateWidget` "/Game/UI_UX/WBP_LoadingScreenPFC.WBP_LoadingScreenPFC_C"))
  (set `self.PFC_Widget` _returnvalue)
  (bind _returnvalue_2 (`|CreateWidget` "/Game/UI_UX/WBP_LoadingScreenPLT.WBP_LoadingScreenPLT_C"))
  (set `self.PLT_Widget` _returnvalue_2)
  (bind _returnvalue_3 (`|CreateWidget` "/Game/UI_UX/WBP_Hub_Score.WBP_Hub_Score_C"))
  (set `self.HubUI` _returnvalue_3)
  (bind _returnvalue_4 (`|CreateWidget` "/Game/UI_UX/WBP_MainMenu.WBP_MainMenu_C"))
  (`UserWidget.AddToViewport` _returnvalue_4 0))

(event `Key|I`
  (params (Key :type "Key Structure"))
  (:`Pressed`
    (`WidgetLayoutLibrary.RemoveAllWidgets`)))

(event `Key|B`
  (params (Key :type "Key Structure"))
  (:`Pressed`
    (`WidgetLayoutLibrary.RemoveAllWidgets`)
    (bind _returnvalue (`|CreateWidget` "/Game/HUD_Game/Sarbacane/WBP_Sarb.WBP_Sarb_C"))
    (`UserWidget.AddToViewport` _returnvalue 0)))

(fn `UserConstructionScript`)